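; BP_BulletDisc is an interactable bullet disc that shows a load/unload prompt when the player character (BP_Alex) is nearby.
; BeginPlay writes the "E" key hint into its WBP_Prompt widget, and actor overlap with Alex shows or hides that widget.
; SetSpriteVisibility applies the inverse of its input to the empty-disc sprite to indicate whether the disc is with the player.
; The load/unload action itself is not handled here.
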(event Custom|SetSpriteVisibility
  (params (newVisibility :type Boolean))
  ;[1 1 1] Set Sprite Visibility to indicate Bullet disc is with player or not
  (Rendering|SetVisibility (Variables|Default|GetBulletDiscEmptySprite) (not newVisibility) false))

(event EventBeginPlay
  ;[1 1 1] Set Interaction Text
  (bind _aswbp_prompt (Utilities|Casting|CastToWBP_Prompt (UserInterface|GetWidget (Variables|Default|GetBulDiscPromptWidget))))
  (Variables|/Game/Stuff/Blueprints/Widgets/WBP_Prompt.WBP_Prompt_C|SetInteractionTextPrompt _aswbp_prompt "E to Load/Unload Bullet Disc"))

(event Collision|EventActorBeginOverlap
  (params (OtherActor :type Actor%20Object%20Reference))
  ;[1 1 1] Set Visibility of Interaction Text
  (Utilities|Casting|CastToBP_Alex OtherActor)
  (Rendering|SetVisibility (Variables|Default|GetBulDiscPromptWidget) true false))

(event EventTick
  (params (DeltaSeconds :type Float%20%28single-precision%29)))

(event Collision|EventActorEndOverlap
  (params (OtherActor :type Actor%20Object%20Reference))
  ;[1 1 1] Set Visibility of Interaction Text
  (Utilities|Casting|CastToBP_Alex OtherActor)
  (Rendering|SetVisibility (Variables|Default|GetBulDiscPromptWidget) false false))

(fn ConstructionScript)