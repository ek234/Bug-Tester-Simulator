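; L3_cc_collbox is a level-three trigger actor that plays a companion cuboid monologue line when the player enters it.
; On BeginPlay it caches the third-person player character and the GI_FullGame game instance.
; An actor overlap from that player calls the game instance's Monologue function with a fixed line and delay, with no guard against repeat triggering.
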(event EventBeginPlay
  (bind _asbp_third_person_character (Utilities|Casting|CastToBP_ThirdPersonCharacter (Game|GetPlayerCharacter 0)))
  (Variables|Default|Setplayer _asbp_third_person_character)
  (bind _asgi_full_game (Utilities|Casting|CastToGI_FullGame (Game|GetGameInstance)))
  (Variables|Default|Setgame _asgi_full_game))

(event Collision|EventActorBeginOverlap
  (params (OtherActor :type Actor%20Object%20Reference))
  (if (== OtherActor (Variables|Default|Getplayer))
    (Default|Monologue (Variables|Default|Getgame) 0 "This must be the companion cuboid mentioned in the logs." 4.0)))

(fn ConstructionScript)