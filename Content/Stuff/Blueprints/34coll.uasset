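; 34coll is a trigger volume that toggles the player character's safe state.
; On BeginPlay it casts player character 0 to BP_Alex and caches it.
; When that character begins overlapping, it sets Issafe to false, and when the overlap ends, it sets Issafe back to true.
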(event EventBeginPlay
  (bind _asbp_alex (Utilities|Casting|CastToBP_Alex (Game|GetPlayerCharacter 0)))
  (Variables|Default|Setalex _asbp_alex))

(event Collision|EventActorEndOverlap
  (params (OtherActor :type Actor%20Object%20Reference))
  (bind _alex (Variables|Default|Getalex))
  (if (== OtherActor _alex)
    (Variables|/Game/Stuff/Blueprints/Alex/BP_Alex.BP_Alex_C|Setissafe _alex true)))

(event Collision|EventActorBeginOverlap
  (params (OtherActor :type Actor%20Object%20Reference))
  (bind _alex (Variables|Default|Getalex))
  (if (== OtherActor _alex)
    (Variables|/Game/Stuff/Blueprints/Alex/BP_Alex.BP_Alex_C|Setissafe _alex false)))

(fn ConstructionScript)