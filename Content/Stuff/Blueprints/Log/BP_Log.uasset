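; BP_Log is an interactable log actor that shows a "Press L to Open Log" prompt when the BP_Alex character is in range.
; BeginPlay writes the prompt text into the WBP_Prompt hosted by its WidgetLogPrompt component.
; Overlap begin and end with BP_Alex toggle that component's visibility and set the character's IsLog flag.
; The actor itself handles no key input and opens no log.
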(event EventBeginPlay
  ;[1 1 1] Set the Interaction Text
  (bind _aswbp_prompt (Utilities|Casting|CastToWBP_Prompt (UserInterface|GetWidget (Variables|Default|GetWidgetLogPrompt))))
  (Variables|/Game/Stuff/Blueprints/Widgets/WBP_Prompt.WBP_Prompt_C|SetInteractionTextPrompt _aswbp_prompt "Press L to Open Log"))

(event Collision|EventActorBeginOverlap
  (params (OtherActor :type Actor%20Object%20Reference))
  ;[1 1 1] Make Text Visible
  (bind _asbp_alex (Utilities|Casting|CastToBP_Alex OtherActor))
  (Variables|/Game/Stuff/Blueprints/Alex/BP_Alex.BP_Alex_C|SetisLog _asbp_alex true)
  (Rendering|SetVisibility (Variables|Default|GetWidgetLogPrompt) true false))

(event Collision|EventActorEndOverlap
  (params (OtherActor :type Actor%20Object%20Reference))
  ;[1 1 1] Make Text Not Visible
  (bind _asbp_alex (Utilities|Casting|CastToBP_Alex OtherActor))
  (Variables|/Game/Stuff/Blueprints/Alex/BP_Alex.BP_Alex_C|SetisLog _asbp_alex false)
  (Rendering|SetVisibility (Variables|Default|GetWidgetLogPrompt) false false))

(fn ConstructionScript)