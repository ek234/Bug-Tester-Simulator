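; Breakable brick wall that cracks progressively with each explosion, then disappears.
; ShowCrack reveals the small or large crack by explosion count, increments it and saves it to GI_FullGame.
; BeginPlay reads that saved count to restore the wall's state.
; CheckBreak hides bricks and cracks and destroys the collision box once ExpToBreak is reached, leaving the actor itself in place.
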(event Custom|ShowCrack
  ;[1 1 1] Show cracks progressively as required
  (switch int (Variables|Default|GetExpCount)
    (:0
      (Variables|Default|SetTarget (Variables|Default|GetSmolCrack))
      (Rendering|SetVisibility (Variables|Default|GetTarget) true false :!label _label)
      (bind _result (Math|Integer|IncrementInt (Variables|Default|GetExpCount))
        (:%20%20
          (Development|PrintString (Utilities|String|ToString(Integer) _result)))))
    (:1
      (Variables|Default|SetTarget (Variables|Default|GetCrack))
      (goto _label))
    (:2
      (bind _result_2 (Math|Integer|IncrementInt (Variables|Default|GetExpCount))
        (:%20%20
          (Development|PrintString (Utilities|String|ToString(Integer) _result_2))
          (CallFunction|CheckBreak)))))
  (bind _asgi_full_game (Utilities|Casting|CastToGI_FullGame (Game|GetGameInstance)))
  (bind _output_get (Variables|/Game/GI_FullGame.GI_FullGame_C|SetExpCount _asgi_full_game (Variables|Default|GetExpCount)))
  (Development|PrintString (Utilities|String|ToString(Integer) _output_get)))

(event Custom|CheckBreak
  ;[1 1 1] Remove Wall Once Enough explosions are done
  (if (>= (Variables|Default|GetExpCount) (Variables|Default|GetExpToBreak))
    (Rendering|SetVisibility (Variables|Default|GetSmolCrack) false false)
    (Rendering|SetVisibility (Variables|Default|GetCrack) false false)
    (Rendering|SetVisibility (Variables|Default|GetBricks) false false)
    (Components|DestroyComponent (Variables|Default|GetColBox))))

(event EventBeginPlay
  (bind _asgi_full_game (Utilities|Casting|CastToGI_FullGame (Game|GetGameInstance)))
  (bind _output_get (Variables|Default|SetExpCount (Variables|/Game/GI_FullGame.GI_FullGame_C|GetExpCount _asgi_full_game)))
  (Development|PrintString "Exp Count is ")
  (Development|PrintString (Utilities|String|ToString(Integer) _output_get))
  (switch int (Variables|Default|GetExpCount)
    (:1
      (Variables|Default|SetTarget (Variables|Default|GetSmolCrack))
      (Rendering|SetVisibility (Variables|Default|GetTarget) true false :!label _label))
    (:2
      (Variables|Default|SetTarget (Variables|Default|GetCrack))
      (goto _label))
    (:3
      (CallFunction|CheckBreak))))

(fn ConstructionScript)