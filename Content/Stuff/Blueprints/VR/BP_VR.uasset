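; BP_VR is a VR pickup actor that grants the VR item to the player character, BP_Alex.
; On BeginPlay it checks GI_FullGame and destroys itself if VrObtained is set and ShouldExplode is not.
; When hit by BP_Alex, it destroys itself, prints a message, sets the character's VR flags and calls its VRObtain function.
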(event EventBeginPlay
  ;[1 1 1] Destroy if already obtained
  (bind _asgi_full_game (Utilities|Casting|CastToGI_FullGame (Game|GetGameInstance)))
  (if (Variables|/Game/GI_FullGame.GI_FullGame_C|GetvrObtained _asgi_full_game)
    (if (not (Variables|/Game/GI_FullGame.GI_FullGame_C|GetshouldExplode _asgi_full_game))
      (Actor|DestroyActor))))

(event EventTick
  (params (DeltaSeconds :type Float%20%28single-precision%29)))

(event Collision|EventHit
  (params (MyComp :type Primitive%20Component%20Object%20Reference) (Other :type Actor%20Object%20Reference) (OtherComp :type Primitive%20Component%20Object%20Reference) (bSelfMoved :type Boolean) (HitLocation :type Vector :default "0, 0, 0") (HitNormal :type Vector :default "0, 0, 0") (NormalImpulse :type Vector :default "0, 0, 0") (Hit :type Hit%20Result%20Structure%20%28by%20ref%29))
  ;[1 1 1] VR Obtain
  (bind _asbp_alex (Utilities|Casting|CastToBP_Alex Other))
  (Actor|DestroyActor)
  (Development|PrintText "VR Obtained!")
  (Variables|/Game/Stuff/Blueprints/Alex/BP_Alex.BP_Alex_C|SetisVR _asbp_alex true)
  (Variables|/Game/Stuff/Blueprints/Alex/BP_Alex.BP_Alex_C|SetvrObtained _asbp_alex true)
  (Default|VRObtain _asbp_alex))

(fn ConstructionScript)