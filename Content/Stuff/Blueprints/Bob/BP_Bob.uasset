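; BP_Bob is a talkable NPC that shows an interact prompt while BP_Alex overlaps it.
; Talk freezes the player and advances a dialog widget by index, restoring walking when the conversation ends.
; First-life talks splice the GameInstance's Bt into an intro before random and closing lines, while later lives skip the intro.
; When CeoComes is set, Bob relocates at BeginPlay and plays a scripted dialog with speaker names and colors.
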(event Custom|RepeatedLifeTalk
  (if (Variables|Default|GetisTalking)
    (Variables|/Game/Stuff/Blueprints/Widgets/WBP_DialogBox.WBP_DialogBox_C|SetDialog (Variables|Default|GetDialogBoxWidget) (Variables|Default|GetEndDialog))
    (bind _result (Math|Integer|IncrementInt (Variables|Default|GetDialogIndex))
      (:%20%20
        (if (> _result 2)
          (Variables|Default|SetisTalking false)
          (Variables|Default|SetDialogIndex 0)
          (Widget|RemovefromParent (Variables|Default|GetDialogBoxWidget))
          (Pawn|Components|CharacterMovement|SetMovementMode (Variables|/Script/Engine.Character|GetCharacterMovement (Variables|Default|GetAs%20BP%20Alex)) "MOVE_Walking" 0))))
    (else
      (bind _returnvalue (UserInterface|CreateWidget "/Game/Stuff/Blueprints/Widgets/WBP_DialogBox.WBP_DialogBox_C" (Game|GetPlayerController 0)))
      (bind _output_get (Variables|Default|SetDialogBoxWidget _returnvalue))
      (UserInterface|Viewport|AddtoViewport _output_get 0)
      (Variables|/Game/Stuff/Blueprints/Widgets/WBP_DialogBox.WBP_DialogBox_C|SetDialog (Variables|Default|GetDialogBoxWidget) (Utilities|Array|Get(acopy) (Variables|Default|GetDialog) (Math|Random|RandomIntegerinRange 0 (- (Utilities|Array|Length (Variables|Default|GetDialog)) 1))))
      (Variables|Default|SetisTalking true)
      (Math|Integer|IncrementInt (Variables|Default|GetDialogIndex)))))

(event Collision|EventActorEndOverlap
  (params (OtherActor :type Actor%20Object%20Reference))
  ;[1 1 1] Stop showing interaction text when player is not nearby
  (Utilities|Casting|CastToBP_Alex OtherActor)
  (Rendering|SetVisibility (Variables|Default|GetPromptWidget) false false))

(event EventBeginPlay
  ;[1 1 1] Set the Interaction Text for when the Player is nearby
  (bind _asgi_full_game (Utilities|Casting|CastToGI_FullGame (Game|GetGameInstance)))
  (Variables|Default|SetGame _asgi_full_game)
  (bind _aswbp_prompt (Utilities|Casting|CastToWBP_Prompt (UserInterface|GetWidget (Variables|Default|GetPromptWidget))))
  (Variables|/Game/Stuff/Blueprints/Widgets/WBP_Prompt.WBP_Prompt_C|SetInteractionTextPrompt _aswbp_prompt "Press E to Interact")
  (bind _asbp_alex (Utilities|Casting|CastToBP_Alex (Game|GetPlayerCharacter 0)))
  (Variables|Default|SetAs%20BP%20Alex _asbp_alex)
  (if (Variables|/Game/GI_FullGame.GI_FullGame_C|Getceo_comes (Variables|Default|GetGame))
    (Transformation|AddActorWorldOffset "-140.000000,-2971.000000,0.000000" false true)))

(event Collision|EventActorBeginOverlap
  (params (OtherActor :type Actor%20Object%20Reference))
  ;[1 1 1] Show interaction text when player is nearby
  (Utilities|Casting|CastToBP_Alex OtherActor)
  (Rendering|SetVisibility (Variables|Default|GetPromptWidget) true false))

(event EventTalk
  (Pawn|Components|CharacterMovement|DisableMovement (Variables|/Script/Engine.Character|GetCharacterMovement (Variables|Default|GetAs%20BP%20Alex)))
  (if (Variables|/Game/GI_FullGame.GI_FullGame_C|Getceo_comes (Variables|Default|GetGame))
    (switch int (Variables|Default|GetDialogIndex)
      (:Default
        (Variables|/Game/Stuff/Blueprints/Widgets/WBP_4throom_diabox.WBP_4throom_diabox_C|SetDialog (Variables|Default|GetDiaBoxWdg4th) (Utilities|Array|Get(acopy) (Variables|Default|Get4RoomDialog) (Variables|Default|GetDialogIndex)))
        (Variables|/Game/Stuff/Blueprints/Widgets/WBP_4throom_diabox.WBP_4throom_diabox_C|SetCharacter (Variables|Default|GetDiaBoxWdg4th) (Utilities|Array|Get(acopy) (Variables|Default|GetCharacterName) (Variables|Default|GetDialogIndex)))
        (Variables|/Game/Stuff/Blueprints/Widgets/WBP_4throom_diabox.WBP_4throom_diabox_C|SetChar%20Color (Variables|Default|GetDiaBoxWdg4th) (Utilities|Array|Get(acopy) (Variables|Default|GetNameColor) (Variables|Default|GetDialogIndex)))
        (Variables|Default|SetisTalking true)
        (bind _result (Math|Integer|IncrementInt (Variables|Default|GetDialogIndex))
          (:%20%20
            (if (== _result (+ (Utilities|Array|Length (Variables|Default|Get4RoomDialog)) 1))
              (Variables|Default|SetisTalking false)
              (Variables|Default|SetDialogIndex 0)
              (Widget|RemovefromParent (Variables|Default|GetDiaBoxWdg4th))
              (Pawn|Components|CharacterMovement|SetMovementMode (Variables|/Script/Engine.Character|GetCharacterMovement (Variables|Default|GetAs%20BP%20Alex)) "MOVE_Walking" 0)))))
      (:0
        (bind _returnvalue (UserInterface|CreateWidget "/Game/Stuff/Blueprints/Widgets/WBP_4throom_diabox.WBP_4throom_diabox_C" (Game|GetPlayerController 0)))
        (bind _output_get (Variables|Default|SetDiaBoxWdg4th _returnvalue))
        (UserInterface|Viewport|AddtoViewport _output_get 0)
        (Variables|/Game/Stuff/Blueprints/Widgets/WBP_4throom_diabox.WBP_4throom_diabox_C|SetDialog (Variables|Default|GetDiaBoxWdg4th) (Utilities|Array|Get(acopy) (Variables|Default|Get4RoomDialog)))
        (Variables|/Game/Stuff/Blueprints/Widgets/WBP_4throom_diabox.WBP_4throom_diabox_C|SetCharacter (Variables|Default|GetDiaBoxWdg4th) (Utilities|Array|Get(acopy) (Variables|Default|GetCharacterName)))
        (Variables|/Game/Stuff/Blueprints/Widgets/WBP_4throom_diabox.WBP_4throom_diabox_C|SetChar%20Color (Variables|Default|GetDiaBoxWdg4th) (Utilities|Array|Get(acopy) (Variables|Default|GetNameColor)))
        (Variables|Default|SetisTalking true)
        (Math|Integer|IncrementInt (Variables|Default|GetDialogIndex))))
    (elif (<= (Variables|/Game/Stuff/Blueprints/Alex/BP_Alex.BP_Alex_C|GetNumLife (Variables|Default|GetAs%20BP%20Alex)) 1)
      (switch int (Variables|Default|GetDialogIndex)
        (:0
          (bind _returnvalue_2 (UserInterface|CreateWidget "/Game/Stuff/Blueprints/Widgets/WBP_DialogBox.WBP_DialogBox_C" (Game|GetPlayerController 0)))
          (bind _output_get_2 (Variables|Default|SetDialogBoxWidget _returnvalue_2))
          (UserInterface|Viewport|AddtoViewport _output_get_2 0)
          (Variables|/Game/Stuff/Blueprints/Widgets/WBP_DialogBox.WBP_DialogBox_C|SetDialog (Variables|Default|GetDialogBoxWidget) (Utilities|Text|ToText(String) (Utilities|String|Append (Utilities|String|GetSubstring (Utilities|String|ToString(Text) (Variables|Default|GetIntroDialog)) 0 18) (Utilities|String|ToString(Integer) (Variables|/Game/GI_FullGame.GI_FullGame_C|Getbt# (Variables|Default|GetGame))) (Utilities|String|GetSubstring (Utilities|String|ToString(Text) (Variables|Default|GetIntroDialog)) 18 50))))
          (Variables|Default|SetisTalking true)
          (Math|Integer|IncrementInt (Variables|Default|GetDialogIndex)))
        (:1
          (Variables|/Game/Stuff/Blueprints/Widgets/WBP_DialogBox.WBP_DialogBox_C|SetDialog (Variables|Default|GetDialogBoxWidget) (Utilities|Array|Get(acopy) (Variables|Default|GetDialog) (Math|Random|RandomIntegerinRange 0 (- (Utilities|Array|Length (Variables|Default|GetDialog)) 1))))
          (Variables|Default|SetisTalking true)
          (Math|Integer|IncrementInt (Variables|Default|GetDialogIndex)))
        (:2
          (Variables|/Game/Stuff/Blueprints/Widgets/WBP_DialogBox.WBP_DialogBox_C|SetDialog (Variables|Default|GetDialogBoxWidget) (Variables|Default|GetEndDialog))
          (Variables|Default|SetisTalking true)
          (Math|Integer|IncrementInt (Variables|Default|GetDialogIndex)))
        (:3
          (if true
            (Variables|Default|SetisTalking false)
            (Variables|Default|SetDialogIndex 0)
            (Widget|RemovefromParent (Variables|Default|GetDialogBoxWidget))
            (Pawn|Components|CharacterMovement|SetMovementMode (Variables|/Script/Engine.Character|GetCharacterMovement (Variables|Default|GetAs%20BP%20Alex)) "MOVE_Walking" 0))))
      (else
        (CallFunction|RepeatedLifeTalk)))))

(fn ConstructionScript)