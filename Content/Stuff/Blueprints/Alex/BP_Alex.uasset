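; BP_Alex is the player-controlled 2D Alex, handling Enhanced Input movement, VR toggling, interaction and a log.
; Talk messages overlapping Bobs or toggles the Bullet Disc, with timed widget prompts reporting pickups and equipment changes.
; The log opens a pausing UI widget, and a debug key appends random entries.
; Explode, with VR equipped, copies state to GI_FullGame and opens ThirdPersonMap, leaving the brick-wall cracking logic unconnected.
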(event Custom|VRObtain
  ;[1 1 1] Obtain VR
  (CallFunction|ShowAlexPromptText "VR Obtained!" 0.5))

(event Custom|SetisLogOpened
  (params (NewVal :type Boolean))
  ;[1 1 1] Log
  (Variables|Default|SetisLogOpened NewVal))

(event Custom|AddLog
  (params (LogString :type String))
  (bind _logtext (Variables|Default|GetLogText))
  ;[1 1 1] Add logs
  (Utilities|Array|AppendArray _logtext (Utilities|Array|MakeArray LogString))
  (Development|PrintString (Utilities|String|ToString(Integer) (Utilities|Array|Length _logtext))))

(event Custom|ShowAlexPromptText
  (params (PromptText :type Text) (PromptDuration :type Float%20%28double-precision%29))
  ;[1 1 1] Event to Show Prompt on Alex
  (bind _aswbp_prompt (Utilities|Casting|CastToWBP_Prompt (UserInterface|GetWidget (Variables|Default|GetWidgetPrompAlex))))
  (Variables|/Game/Stuff/Blueprints/Widgets/WBP_Prompt.WBP_Prompt_C|SetInteractionTextPrompt _aswbp_prompt PromptText)
  (Rendering|SetVisibility (Variables|Default|GetWidgetPrompAlex) true false)
  (Utilities|FlowControl|Delay PromptDuration)
  (Rendering|SetVisibility (Variables|Default|GetWidgetPrompAlex) false false))

(event Custom|UpdateGIfrom2D
  (bind _gi_full_game (Variables|Default|GetGI%20Full%20Game))
  (Variables|/Game/GI_FullGame.GI_FullGame_C|SetvrObtained _gi_full_game (Variables|Default|GetvrObtained))
  (Variables|/Game/GI_FullGame.GI_FullGame_C|SetisVR _gi_full_game (Variables|Default|GetisVR))
  (Variables|/Game/GI_FullGame.GI_FullGame_C|SethaveBulDisc? _gi_full_game (Variables|Default|GethaveBulDisc?))
  (bind _output_get (Variables|Default|SetLocation (Transformation|GetActorLocation)))
  (Variables|/Game/GI_FullGame.GI_FullGame_C|SetAlexLocation _gi_full_game _output_get)
  (Variables|/Game/GI_FullGame.GI_FullGame_C|SetLogText _gi_full_game (Variables|Default|GetLogText))
  (Variables|/Game/GI_FullGame.GI_FullGame_C|SetgoToRoom _gi_full_game (Variables|Default|GetgoToRoom)))

(event Input|EnhancedActionEvents|EnhancedInputActionIA_Log
  (params (ActionValue :type Boolean) (ElapsedSeconds :type Float%20%28double-precision%29) (TriggeredSeconds :type Float%20%28double-precision%29) (InputAction :type Input%20Action%20Object%20Reference :default "/Game/Stuff/Blueprints/Alex/Input/IA_Log.IA_Log"))
  (bind _playercontroller (Variables|Default|GetPlayerController))
  ;[1 1 1] Log
  (:Started
    (if (Variables|Default|GetisLog)
      (if (not (Variables|Default|GetisLogOpened))
        (Variables|Default|SetisLogOpened true)
        (Development|PrintText "Opened Log")
        (bind _returnvalue (UserInterface|CreateWidget "/Game/Stuff/Blueprints/Widgets/WBP_Log.WBP_Log_C" _playercontroller))
        (bind _output_get (Variables|Default|SetLogWidget _returnvalue))
        (UserInterface|Viewport|AddtoViewport _output_get 0)
        (Input|SetInputModeGameandUI _playercontroller (Variables|Default|GetLogWidget) "DoNotLock" true false)
        (Variables|/Script/Engine.PlayerController|SetbShowMouseCursor _playercontroller true)
        (Game|SetGamePaused true)))))

(event Input|EnhancedActionEvents|EnhancedInputActionIA_VR
  (params (ActionValue :type Boolean) (ElapsedSeconds :type Float%20%28double-precision%29) (TriggeredSeconds :type Float%20%28double-precision%29) (InputAction :type Input%20Action%20Object%20Reference :default "/Game/Stuff/Blueprints/Alex/Input/IA_VR.IA_VR"))
  ;[1 1 1] VR Equip/Unequip
  (:Started
    (if (Variables|Default|GetvrObtained)
      (if (Variables|Default|GetisVR)
        (Variables|Default|SetisVR false)
        (Development|PrintText "VR Unequipped")
        (CallFunction|ShowAlexPromptText "VR Unequipped!" 0.5)
        (else
          (Variables|Default|SetisVR true)
          (Development|PrintText "VR Equipped")
          (if (Variables|Default|GethaveBulDisc?)
            (CallFunction|ShowAlexPromptText "VR Equipped with Bullet Disc!" 0.5)
            (else
              (CallFunction|ShowAlexPromptText "VR Equipped!" 0.5))))))))

(event Input|EnhancedActionEvents|EnhancedInputActionIA_Alex
  (params (ActionValue :type Vector%202D%20Structure) (ElapsedSeconds :type Float%20%28double-precision%29) (TriggeredSeconds :type Float%20%28double-precision%29) (InputAction :type Input%20Action%20Object%20Reference :default "/Game/Stuff/Blueprints/Alex/Input/IA_Alex.IA_Alex"))
  ;[0.01042 0 0] Add Movement
  (:Triggered
    (Pawn|Input|AddMovementInput "0.500000,0.000000,0.000000" (.x ActionValue) false)
    (Pawn|Input|AddMovementInput "0.000000,-0.500000,0.000000" (.y ActionValue) false)
    (Variables|Default|SetDirectionality (Math|Vector2D|MakeVector2D (.x ActionValue) (.y ActionValue))))
  (:Started
    (Variables|Default|SetisHoldingMove? true))
  (:Completed
    (Variables|Default|SetisHoldingMove? false)))

(event Input|EnhancedActionEvents|EnhancedInputActionIA_Explode
  (params (ActionValue :type Boolean) (ElapsedSeconds :type Float%20%28double-precision%29) (TriggeredSeconds :type Float%20%28double-precision%29) (InputAction :type Input%20Action%20Object%20Reference :default "/Game/Stuff/Blueprints/Alex/Input/IA_Explode.IA_Explode"))
  ;[1 1 1] Explosion
  (:Started
    (if (Variables|Default|GetisVR)
      (CallFunction|UpdateGIfrom2D)
      (Game|OpenLevel(byObjectReference) "/Game/ThirdPerson/Maps/ThirdPersonMap.ThirdPersonMap" false))))

(event Input|EnhancedActionEvents|EnhancedInputActionIA_Talk
  (params (ActionValue :type Boolean) (ElapsedSeconds :type Float%20%28double-precision%29) (TriggeredSeconds :type Float%20%28double-precision%29) (InputAction :type Input%20Action%20Object%20Reference :default "/Game/Stuff/Blueprints/Alex/Input/IA_Talk.IA_Talk"))
  ;[1 1 1] Talk to Bob or Interact With Bullet Disc
  (:Started
    (for _array_element (Collision|GetOverlappingActors "/Game/Stuff/Blueprints/Bob/BP_Bob.BP_Bob_C" :!class /Script/Engine.Actor)
      (if (Utilities|DoesObjectImplementInterface _array_element "/Game/Stuff/Blueprints/Bob/BPI_BobTalk.BPI_BobTalk_C")
        (Class|BPIBobTalk|Talk(Message) _array_element)))
    (for _array_element_2 (Collision|GetOverlappingActors "/Game/Stuff/Blueprints/BulletDisk/BP_BulletDisc.BP_BulletDisc_C" :!class /Script/Engine.Actor)
      (bind _asbp_bullet_disc (Utilities|Casting|CastToBP_BulletDisc _array_element_2))
      (Default|SetSpriteVisibility _asbp_bullet_disc (Variables|Default|GethaveBulDisc?))
      (Variables|Default|SethaveBulDisc? (not (Variables|Default|GethaveBulDisc?)))
      (Development|PrintString (Utilities|String|ToString(Boolean) (Variables|Default|GethaveBulDisc?)))
      (if (Variables|Default|GethaveBulDisc?)
        (CallFunction|ShowAlexPromptText "Bullet Disc Obtained!" 0.5)
        (else
          (CallFunction|ShowAlexPromptText "Bullet Disc Removed!" 0.5))))))

(event EventBeginPlay
  ;[0.2135 0.07919 0] Setting up taking of input
  (bind _asgi_full_game (Utilities|Casting|CastToGI_FullGame (Game|GetGameInstance)))
  (Variables|Default|SetGI%20Full%20Game _asgi_full_game)
  (bind _asplayer_controller (Utilities|Casting|CastToPlayerController (Pawn|GetController)))
  (Input|AddMappingContext (PlayerController|LocalPlayerSubsystems|GetEnhancedInputLocalPlayerSubsystem _asplayer_controller) "/Game/Stuff/Blueprints/Alex/Input/IMC_Alex.IMC_Alex" 0 "(bIgnoreAllPressedKeysUntilRelease=True,bForceImmediately=False,bNotifyUserSettings=False)")
  (Variables|Default|SetgoToRoom 1)
  (Variables|Default|SetPlayerController (Game|GetPlayerController 0)))

(event Input|KeyboardEvents|I
  (params (Key :type Key%20Structure :default "None"))
  (:Pressed
    (CallFunction|AddLog (Utilities|String|Append "This is random entry with num = " (Utilities|String|ToString(Integer) (Math|Random|RandomInteger 1000))))))

(fn ConstructionScript)