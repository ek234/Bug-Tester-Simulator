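; An interactable console actor that opens a login-style widget when the third-person character is within its box trigger.
; OpenClose, if in range, pauses the game, shows ConsoleWidgetBP and switches to UI-only input with a mouse cursor.
; Leaving the box copies Username and Password from the widget, substituting defaults when empty, then calls CallUpdateUsernamesGlobally.
; StopInteract restores game input and hides the cursor but does not unpause, and nothing here runs it.
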(event OnComponentEndOverlap(Box)
  (params (OverlappedComponent :type Primitive%20Component%20Object%20Reference) (OtherActor :type Actor%20Object%20Reference) (OtherComp :type Primitive%20Component%20Object%20Reference) (OtherBodyIndex :type Integer))
  (Utilities|Casting|CastToBP_ThirdPersonCharacter OtherActor)
  (Variables|Default|SetinRange? false)
  (if (Utilities|Enum|Equal(Enum) (Utilities|String|ToString(Text) (Variables|/Game/ExternalAssets/console/consoleWidgetBP.consoleWidgetBP_C|Getusername (stale Custom|StartInteract _returnvalue))) "")
    (Variables|Default|SetUsername "TESTER#0")
    (else
      (Variables|Default|SetUsername (Variables|/Game/ExternalAssets/console/consoleWidgetBP.consoleWidgetBP_C|Getusername (stale Custom|StartInteract _returnvalue)))))
  (if (Utilities|Enum|Equal(Enum) (Utilities|String|ToString(Text) (Variables|/Game/ExternalAssets/console/consoleWidgetBP.consoleWidgetBP_C|Getpassword (stale Custom|StartInteract _returnvalue))) "")
    (Variables|Default|SetPassword "run_away")
    (else
      (Variables|Default|SetPassword (Variables|/Game/ExternalAssets/console/consoleWidgetBP.consoleWidgetBP_C|Getpassword (stale Custom|StartInteract _returnvalue)))))
  (Default|CallUpdateUsernamesGlobally))

(event OnComponentBeginOverlap(Box)
  (params (OverlappedComponent :type Primitive%20Component%20Object%20Reference) (OtherActor :type Actor%20Object%20Reference) (OtherComp :type Primitive%20Component%20Object%20Reference) (OtherBodyIndex :type Integer) (bFromSweep :type Boolean) (SweepResult :type Hit%20Result%20Structure%20%28by%20ref%29))
  (Utilities|Casting|CastToBP_ThirdPersonCharacter OtherActor)
  (Variables|Default|SetinRange? true))

(event Custom|StopInteract
  (bind _returnvalue (Game|GetPlayerController 0))
  (Input|SetInputModeGameOnly _returnvalue false)
  (Variables|/Script/Engine.PlayerController|SetbShowMouseCursor _returnvalue false))

(event Custom|StartInteract
  (Game|SetGamePaused true)
  (bind _returnvalue (UserInterface|CreateWidget "/Game/ExternalAssets/console/consoleWidgetBP.consoleWidgetBP_C"))
  (UserInterface|Viewport|AddtoViewport _returnvalue 0)
  (Input|SetInputModeUIOnly (Game|GetPlayerController 0) _returnvalue "DoNotLock" false)
  (Variables|/Script/Engine.PlayerController|SetbShowMouseCursor (Game|GetPlayerController 0) true)
  (Variables|Default|SetisInteracting? true))

(event Custom|Toggle%20Interact
  (Development|PrintString "console")
  (CallFunction|StartInteract))

(event EventOpenClose
  (if (Variables|Default|GetinRange?)
    (CallFunction|ToggleInteract)))

(fn ConstructionScript)